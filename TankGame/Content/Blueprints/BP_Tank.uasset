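; BP_Tank is the player-controlled tank pawn, driven by separate left and right track throttle inputs.
; On BeginPlay it hands its barrel and turret to the TankAiming component, which also handles the Fire input.
; Look input yaws the Scene component and pitches the SpringArm within a clamped range to orbit the view.
; The left throttle also prints its axis value to screen.
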(event `InputAction|Fire`
  (params (Key :type "Key Structure"))
  (:`Pressed`
    (`TankAimingComponent.Fire` (`self.TankAiming`))))

(event `self.ReceiveBeginPlay`
  (`TankAimingComponent.Initialise` (`self.TankAiming`) (`self.TankBarrel`) (`self.TankTurret`)))

(event `InputAxis|LeftTrackThottle`
  (params (AxisValue :type "Float (single-precision)"))
  (`TankTrack.SetThrottle` (`self.LeftTrack`) AxisValue)
  (`KismetSystemLibrary.PrintString` (`KismetStringLibrary.Conv_DoubleToString` AxisValue)))

(event `InputAxis|RightTrackThottle`
  (params (AxisValue :type "Float (single-precision)"))
  (`TankTrack.SetThrottle` (`self.RightTrack`) AxisValue))

(event `InputAxis|LookH`
  (params (AxisValue :type "Float (single-precision)"))
  ;[1 1 1] 控制左右旋转
  (`SceneComponent.K2_AddRelativeRotation` (`self.Scene`) (`KismetMathLibrary.MakeRotator` 0.0 0.0 AxisValue) false false) ; add
)

(event `InputAxis|LookV`
  (params (AxisValue :type "Float (single-precision)"))
  (bind (_relativerotation_roll _relativerotation_pitch _relativerotation_yaw) (`KismetMathLibrary.BreakRotator` (`SceneComponent.RelativeRotation` (`self.SpringArm`))))
  ;[1 1 1] 控制上下旋转】
  (`SceneComponent.K2_SetRelativeRotation` (`self.SpringArm`) (`KismetMathLibrary.MakeRotator` _relativerotation_roll (`KismetMathLibrary.FClamp` (+ AxisValue _relativerotation_pitch) -40.0 5.0) _relativerotation_yaw) false false) ; set
)

(fn `UserConstructionScript`)